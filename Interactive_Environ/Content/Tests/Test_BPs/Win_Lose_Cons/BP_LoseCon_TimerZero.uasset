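; Functional test Blueprint for the lose condition where a countdown timer runs out.
; Each Tick subtracts world delta seconds from Countdown, clamped at zero, then enters a two-second Delay.
; After the delay, it calls FinishTest with a lose message if Countdown equals zero, otherwise a failed message.
; Both outcomes report the Default test result, so only the message distinguishes them.
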(event Custom|CountdownEvent
  (Variables|Default|SetCountdown (Math|Float|Clamp(Float) (- (Variables|Default|GetCountdown) (Utilities|Time|GetWorldDeltaSeconds)) 0.0 (Variables|Default|GetCountdown)))
  (Utilities|FlowControl|Delay 2.0)
  (if (== (Variables|Default|GetCountdown) 0.0)
    (Class|FunctionalTest|FinishTest "Default" "you lose, due to timer running out")
    (else
      (Class|FunctionalTest|FinishTest "Default" "failed"))))

(event EventTick
  (params (DeltaSeconds :type Float%20%28single-precision%29))
  (CallFunction|CountdownEvent))

(fn ConstructionScript)