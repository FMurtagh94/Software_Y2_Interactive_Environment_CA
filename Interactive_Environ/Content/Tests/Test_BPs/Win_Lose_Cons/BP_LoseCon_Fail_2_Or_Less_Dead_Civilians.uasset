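; BP_LoseCon_Fail_2_Or_Less_Dead_Civilians is a test Blueprint for the civilian-death lose condition.
; Each tick it checks whether CivilianCount equals three and, if so, finishes the test with a lose message.
; Otherwise it decrements a clamped Countdown by world delta time and finishes at zero, reporting fewer than three dead.
; Both outcomes pass a Default test result, and nothing here updates CivilianCount.
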(event Custom|CountdownEvent
  (if (== (Variables|Default|GetcivilianCount) 3)
    (Class|FunctionalTest|FinishTest "Default" "3 dead civilians, you lose")
    (else
      (Variables|Default|SetCountdown (Math|Float|Clamp(Float) (- (Variables|Default|GetCountdown) (Utilities|Time|GetWorldDeltaSeconds)) 0.0 (Variables|Default|GetCountdown)))
      (if (== (Variables|Default|GetCountdown) 0.0)
        (Class|FunctionalTest|FinishTest "Default" "There are less than 3 civilians dead")))))

(event EventTick
  (params (DeltaSeconds :type Float%20%28single-precision%29))
  (CallFunction|CountdownEvent))

(fn ConstructionScript)