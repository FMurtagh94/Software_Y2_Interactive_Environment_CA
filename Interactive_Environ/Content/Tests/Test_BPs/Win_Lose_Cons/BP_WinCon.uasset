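; Functional test Blueprint for a win condition, checking whether all enemies die before a countdown expires.
; Each Tick calls CountdownEvent, which ends the test with a win message if EnemyCount is zero.
; Otherwise it subtracts world delta seconds from Countdown, clamped at zero, and finishes with a "Fail" message on reaching zero.
; Both outcomes pass the Default test result, differing only in message.
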(event Custom|CountdownEvent
  (if (== (Variables|Default|GetEnemyCount) 0)
    (Class|FunctionalTest|FinishTest "Default" "Enemies are all dead, you win!")
    (else
      (Variables|Default|SetCountdown (Math|Float|Clamp(Float) (- (Variables|Default|GetCountdown) (Utilities|Time|GetWorldDeltaSeconds)) 0.0 (Variables|Default|GetCountdown)))
      (if (== (Variables|Default|GetCountdown) 0.0)
        (Class|FunctionalTest|FinishTest "Default" "Fail")))))

(event EventTick
  (params (DeltaSeconds :type Float%20%28single-precision%29))
  (CallFunction|CountdownEvent))

(fn ConstructionScript)