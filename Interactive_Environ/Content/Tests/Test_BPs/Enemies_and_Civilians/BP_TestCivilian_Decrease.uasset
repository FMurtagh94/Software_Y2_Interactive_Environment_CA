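; Functional test that checks the civilian count decreases when a BP_MovingCivilian dies.
; On StartTest it records the number of civilians in the level, has the referenced BP_ThirdPersonCharacter spawn a projectile, then binds to each civilian's OnDeath.
; A death decrements the count and finishes the test with a success or failure message, though both branches pass the Default result.
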(event Custom|CivilDeath_Event
  (Math|Integer|DecrementInt (Variables|Default|GetCivilCount)
    (:%20%20
      (if (> (Variables|Default|GetmaxCivilCount) (Variables|Default|GetCivilCount))
        (Class|FunctionalTest|FinishTest "Default" "1 civilan is removed")
        (else
          (Class|FunctionalTest|FinishTest "Default" "failure"))))))

(event EventStartTest
  (bind _outactors (Actor|GetAllActorsOfClass "/Game/Blueprints/Game_BPs/BP_MovingCivilian.BP_MovingCivilian_C"))
  (Variables|Default|SetCivilCount (Utilities|Array|Length _outactors))
  (Variables|Default|SetmaxCivilCount (Utilities|Array|Length _outactors))
  (bind _asbp_third_person_character (Utilities|Casting|CastToBP_ThirdPersonCharacter (Variables|Default|GetCharRef)))
  (Default|SpawnProjectile _asbp_third_person_character)
  (for _array_element _outactors
    (EventDispatchers|BindEventtoOnDeath _array_element (delegate Custom|CivilDeath_Event))))

(fn ConstructionScript)