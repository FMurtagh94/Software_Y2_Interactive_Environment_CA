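; BP_TestEnemy_Decrease is a functional test that checks that the enemy count drops when an enemy dies.
; On test start it records the number of BP_MovingEnemy actors, makes the referenced third-person character spawn a projectile, then binds to every enemy's OnDeath.
; A death decrements the count and finishes the test with the Default result once it falls below the starting total.
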(event Custom|OnDeath_Event
  (Math|Integer|DecrementInt (Variables|Default|GetEnemyCount)
    (:%20%20
      (if (< (Variables|Default|GetEnemyCount) (Variables|Default|GetMaxEnemyCount))
        (Class|FunctionalTest|FinishTest "Default" "1 enemy is removed")))))

(event EventStartTest
  (bind _outactors (Actor|GetAllActorsOfClass "/Game/Blueprints/Game_BPs/BP_MovingEnemy.BP_MovingEnemy_C"))
  (bind _output_get (Variables|Default|SetEnemyCount (Utilities|Array|Length _outactors)))
  (Variables|Default|SetMaxEnemyCount _output_get)
  (bind _asbp_third_person_character (Utilities|Casting|CastToBP_ThirdPersonCharacter (Variables|Default|GetCharRef)))
  (Default|SpawnProjectile _asbp_third_person_character)
  (for _array_element _outactors
    (EventDispatchers|AssignOnDeath _array_element (delegate Custom|OnDeath_Event))))

(fn ConstructionScript)