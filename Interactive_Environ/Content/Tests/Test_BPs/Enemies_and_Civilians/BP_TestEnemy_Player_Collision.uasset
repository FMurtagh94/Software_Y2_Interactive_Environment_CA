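; BP_TestEnemy_Player_Collision is a functional test that checks whether an enemy stays alive when the player character runs into it.
; Each Tick pushes the referenced character along its forward vector, then a 1.5-second Delay leads to the check.
; The check compares the enemy kill reference's current and maximum enemy counts to choose the finish message.
; Both branches finish with the Default result, so only the message distinguishes survival from death.
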(event EventTick
  (params (DeltaSeconds :type Float%20%28single-precision%29))
  (bind _enemykillref (Variables|Default|GetenemyKillRef))
  (bind _charref (Variables|Default|GetCharRef))
  (Pawn|Input|AddMovementInput _charref (Transformation|GetActorForwardVector _charref) 1.0 false)
  (Utilities|FlowControl|Delay 1.5)
  (if (== (Variables|/Game/Blueprints/Game_BPs/HUD/WBP_EnemiesRemaining.WBP_EnemiesRemaining_C|GetMaxEnemyCount _enemykillref) (Variables|/Game/Blueprints/Game_BPs/HUD/WBP_EnemiesRemaining.WBP_EnemiesRemaining_C|GetEnemyCount _enemykillref))
    (Class|FunctionalTest|FinishTest "Default" "Enemy stays alive when in contact with player character.")
    (else
      (Class|FunctionalTest|FinishTest "Default" "Enemy died"))))

(fn ConstructionScript)