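; BP_MovingEnemy is an enemy actor that shuttles back and forth and dies when any actor overlaps it.
; Tick offsets it by Direction times Speed without sweep or delta-time scaling, so movement depends on frame rate.
; A looping timer started on BeginPlay negates Direction every TimeToChange seconds.
; An overlap triggers Die, which calls the OnDeath dispatcher before destroying the actor.
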(event Custom|Die
  (Default|CallOnDeath)
  (Actor|DestroyActor))

(event Custom|CustomEvent
  (Variables|Default|SetDirection (* (Variables|Default|GetDirection) -1.0)))

(event EventBeginPlay
  (Utilities|Time|SetTimerbyEvent (delegate Custom|CustomEvent) (Variables|Default|GetTimeToChange) true))

(event Collision|EventActorBeginOverlap
  (params (OtherActor :type Actor%20Object%20Reference))
  (CallFunction|Die))

(event EventTick
  (params (DeltaSeconds :type Float%20%28single-precision%29))
  (Transformation|AddActorWorldOffset (* (Variables|Default|GetDirection) (Variables|Default|GetSpeed))))

(fn ConstructionScript)