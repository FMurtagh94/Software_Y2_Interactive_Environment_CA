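; Functional test Blueprint for ammo decrease, built around checking that Ammo equals zero.
; StartTest calls a GetController helper, which casts the first player pawn's controller to TestPlayerController, then sets Ammo directly to zero.
; The equality assertion and the FinishTest success call are disconnected from execution, so the test never reports a result itself.
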(event EventPrepareTest)

(event EventStartTest
  (CallFunction|GetController)
  (Variables|Default|SetAmmo 0))

(event EventTick
  (params (DeltaSeconds :type Float%20%28single-precision%29)))

(fn ConstructionScript)

(fn GetController
  (bind _astest_player_controller (Utilities|Casting|CastToTestPlayerController (Pawn|GetController (Game|Player|GetPlayerPawn 0)))
    (:then
      _)
    (:CastFailed
      _))
  (return _astest_player_controller))