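; BP_MovementTest is a functional test that checks whether a character can traverse a course to the other side.
; Tick constantly feeds forward movement input while StartTest plays a timed script of 90-degree turns and jumps through chained delays.
; The test succeeds when the character overlaps the Trigger actor; the Blueprint itself has no explicit failure branch.
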(event OnActorBeginOverlap(Trigger)
  (params (OverlappedActor :type Actor%20Object%20Reference) (OtherActor :type Actor%20Object%20Reference))
  (if (== OtherActor (Variables|Default|GetCharacter))
    (Class|FunctionalTest|FinishTest "Succeeded" "Player made it to the other side!")))

(event EventPrepareTest)

(event EventStartTest
  (Utilities|FlowControl|Delay 1.6)
  (Transformation|AddActorLocalRotation (Variables|Default|GetCharacter) "0.000000,90.000000,0.000000" false false)
  (Utilities|FlowControl|Delay 0.5)
  (Transformation|AddActorLocalRotation (Variables|Default|GetCharacter) "0.000000,-90.000000,0.000000" false false)
  (Utilities|FlowControl|Delay 1.5)
  (Transformation|AddActorLocalRotation (Variables|Default|GetCharacter) "0.000000,-90.000000,0.000000" false false)
  (Utilities|FlowControl|Delay 1.0)
  (Transformation|AddActorLocalRotation (Variables|Default|GetCharacter) "0.000000,90.000000,0.000000" false false)
  (Utilities|FlowControl|Delay 0.5)
  (Character|Jump (Variables|Default|GetCharacter))
  (Utilities|FlowControl|Delay 0.8)
  (Character|Jump (Variables|Default|GetCharacter))
  (Utilities|FlowControl|Delay 0.5)
  (Transformation|AddActorLocalRotation (Variables|Default|GetCharacter) "0.000000,90.000000,0.000000" false false)
  (Utilities|FlowControl|Delay 0.5)
  (Character|Jump (Variables|Default|GetCharacter))
  (Utilities|FlowControl|Delay 0.5)
  (Transformation|AddActorLocalRotation (Variables|Default|GetCharacter) "0.000000,-90.000000,0.000000" false false)
  (Utilities|FlowControl|Delay 0.5)
  (Character|Jump (Variables|Default|GetCharacter)))

(event EventTick
  (params (DeltaSeconds :type Float%20%28single-precision%29))
  (bind _character (Variables|Default|GetCharacter))
  (Pawn|Input|AddMovementInput _character (Transformation|GetActorForwardVector _character) 1.0 false))

(fn ConstructionScript)