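; Functional test that checks BP_ThirdPersonCharacter's DecreaseAmmo does not take Ammo below zero.
; StartTest casts CharRef to the character, sets Ammo to 0, calls DecreaseAmmo and asserts the value is still 0.
; It finishes as Succeeded on a match, with no explicit finish for a failed cast or assertion.
; A GetController helper casts the player's controller to TestPlayerController but is not called here.
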(event EventPrepareTest)

(event EventStartTest
  (bind _asbp_third_person_character (Utilities|Casting|CastToBP_ThirdPersonCharacter (Variables|Default|GetCharRef)))
  (Variables|/Game/ThirdPerson/Blueprints/BP_ThirdPersonCharacter.BP_ThirdPersonCharacter_C|SetAmmo _asbp_third_person_character 0)
  (Default|DecreaseAmmo _asbp_third_person_character)
  (bind _returnvalue (Class|FunctionalTest|AssertEqualInt (Variables|/Game/ThirdPerson/Blueprints/BP_ThirdPersonCharacter.BP_ThirdPersonCharacter_C|GetAmmo _asbp_third_person_character)))
  (if _returnvalue
    (Class|FunctionalTest|FinishTest "Succeeded" "Ammo is 0")))

(event EventTick
  (params (DeltaSeconds :type Float%20%28single-precision%29)))

(fn ConstructionScript)

(fn GetController
  (bind _astest_player_controller (Utilities|Casting|CastToTestPlayerController (Pawn|GetController (Game|Player|GetPlayerPawn 0)))
    (:then
      _)
    (:CastFailed
      _))
  (return _astest_player_controller))