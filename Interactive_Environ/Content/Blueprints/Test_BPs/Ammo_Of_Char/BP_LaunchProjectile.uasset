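; BP_LaunchProjectile is a functional test that checks that the third-person character launches a projectile.
; On test start it counts BP_Projectile actors, calls SpawnProjectile on the referenced character, then asserts that the count has risen by exactly one.
; It finishes as succeeded when the assert passes; a failed assert or character cast never reaches a finish call.
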(event EventStartTest
  (bind _outactors (Actor|GetAllActorsOfClass "/Game/Blueprints/Game_BPs/BP_Projectile.BP_Projectile_C"))
  (Variables|Default|SetPreSpawn (Utilities|Array|Length _outactors))
  (bind _asbp_third_person_character (Utilities|Casting|CastToBP_ThirdPersonCharacter (Variables|Default|GetCharRef)))
  (Default|SpawnProjectile _asbp_third_person_character)
  (bind _outactors_2 (Actor|GetAllActorsOfClass "/Game/Blueprints/Game_BPs/BP_Projectile.BP_Projectile_C"))
  (bind _returnvalue (Class|FunctionalTest|AssertEqualInt (Utilities|Array|Length _outactors_2) (+ (Variables|Default|GetPreSpawn) 1)))
  (if _returnvalue
    (Class|FunctionalTest|FinishTest "Succeeded" "Projectile Launched!")))

(fn ConstructionScript)