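; Ammo pickup actor that oscillates back and forth and refills the player's ammo on contact.
; Box overlap with BP_ThirdPersonCharacter adds RefillAmmo to its Ammo, destroys the pickup and prints a hardcoded gain message.
; A looping timer negates Direction every TimeToChange seconds, while Tick offsets the actor by Direction times Speed without sweep or delta-time scaling.
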(event OnComponentBeginOverlap(Box)
  (params (OverlappedComponent :type Primitive%20Component%20Object%20Reference) (OtherActor :type Actor%20Object%20Reference) (OtherComp :type Primitive%20Component%20Object%20Reference) (OtherBodyIndex :type Integer) (bFromSweep :type Boolean) (SweepResult :type Hit%20Result%20Structure%20%28by%20ref%29))
  (bind _asbp_third_person_character (Utilities|Casting|CastToBP_ThirdPersonCharacter OtherActor))
  (Variables|/Game/ThirdPerson/Blueprints/BP_ThirdPersonCharacter.BP_ThirdPersonCharacter_C|SetAmmo _asbp_third_person_character (+ (Variables|/Game/ThirdPerson/Blueprints/BP_ThirdPersonCharacter.BP_ThirdPersonCharacter_C|GetAmmo _asbp_third_person_character) (Variables|Default|GetRefillAmmo)))
  (Actor|DestroyActor)
  (Development|PrintString "Gained 6 ammo!!"))

(event Custom|ChangeDir
  (Variables|Default|SetDirection (* (Variables|Default|GetDirection) -1.0)))

(event EventBeginPlay
  (Utilities|Time|SetTimerbyEvent (delegate Custom|ChangeDir) (Variables|Default|GetTimeToChange) true))

(event EventTick
  (params (DeltaSeconds :type Float%20%28single-precision%29))
  (Transformation|AddActorWorldOffset (* (Variables|Default|GetDirection) (Variables|Default|GetSpeed))))

(fn ConstructionScript)