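; Interactive moving platform that starts moving once the third-person player character overlaps its box.
; BeginPlay caches the player character and starts a looping timer that flips the travel direction every TimeToChange seconds.
; Tick and the overlap event share one check, offsetting the platform by Direction times Speed, unscaled by delta time and without sweep.
; The check reads the last overlap's actor, and no end-overlap event halts movement.
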(event OnComponentBeginOverlap(Box)
  (params (OverlappedComponent :type Primitive%20Component%20Object%20Reference) (OtherActor :type Actor%20Object%20Reference) (OtherComp :type Primitive%20Component%20Object%20Reference) (OtherBodyIndex :type Integer) (bFromSweep :type Boolean) (SweepResult :type Hit%20Result%20Structure%20%28by%20ref%29))
  (if (== OtherActor (Variables|Default|GetAs%20BP%20Third%20Person%20Character))
    (Transformation|AddActorWorldOffset (* (Variables|Default|GetDirection) (Variables|Default|GetSpeed)))))

(event Custom|ChangeDir
  (Variables|Default|SetDirection (* (Variables|Default|GetDirection) -1.0)))

(event EventBeginPlay
  (bind _asbp_third_person_character (Utilities|Casting|CastToBP_ThirdPersonCharacter (Game|GetPlayerCharacter 0)))
  (Variables|Default|SetAs%20BP%20Third%20Person%20Character _asbp_third_person_character)
  (Utilities|Time|SetTimerbyEvent (delegate Custom|ChangeDir) (Variables|Default|GetTimeToChange) true))

(event Collision|EventActorBeginOverlap
  (params (OtherActor :type Actor%20Object%20Reference)))

(event EventTick
  (params (DeltaSeconds :type Float%20%28single-precision%29))
  (if (== (stale OnComponentBeginOverlap(Box) OtherActor) (Variables|Default|GetAs%20BP%20Third%20Person%20Character))
    (Transformation|AddActorWorldOffset (* (Variables|Default|GetDirection) (Variables|Default|GetSpeed)))))

(fn ConstructionScript)